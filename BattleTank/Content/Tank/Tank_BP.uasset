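; Player-controllable tank Blueprint that binds driving, aiming and firing input.
; Driving axes either set each track's throttle directly or send forward and turn intents to TankMovement, which receives both tracks on BeginPlay.
; Aim axes rotate the azimuth gimbal and spring arm, scaled by delta time, rather than rotating turret or barrel directly.
; BeginPlay also registers barrel and turret references; left mouse calls Fire.
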(event EventBeginPlay
  (Class|Tank|SetBarrelReference (Variables|Default|GetBarrel))
  (Class|Tank|SetTurretReference (Variables|Default|GetTurret))
  (Class|TankMovementComponent|Initialise (Variables|Default|GetTankMovement) (Variables|Default|GetLeftTrack) (Variables|Default|GetRightTrack)))

(event Input|AxisEvents|InputAxisAim_Azimute
  (params (AxisValue :type Float%20%28single-precision%29))
  ;[1 1 1] Aim Input Binding
  (Transformation|AddLocalRotation (Variables|Default|GetAzimuth_Gimbal) (Math|Rotator|MakeRotator 0.0 0.0 (* AxisValue (Utilities|Time|GetWorldDeltaSeconds) 1e+01)) false false))

(event Input|AxisEvents|InputAxisAim_Altitude
  (params (AxisValue :type Float%20%28single-precision%29))
  ;[1 1 1] Aim Input Binding
  (Transformation|AddLocalRotation (Variables|Default|GetSpringArm) (Math|Rotator|MakeRotator 0.0 (* AxisValue (Utilities|Time|GetWorldDeltaSeconds) 1e+01) 0.0) false false))

(event Input|AxisEvents|InputAxisThrowLeft
  (params (AxisValue :type Float%20%28single-precision%29))
  ;[1 1 1] Movement Input Binding
  (Class|TankMovementComponent|IntendTurnLeft (Variables|Default|GetTankMovement) AxisValue))

(event Input|AxisEvents|InputAxisLeftTrackThrottle
  (params (AxisValue :type Float%20%28single-precision%29))
  ;[1 1 1] Movement Input Binding
  (Class|TankTrack|SetThrottle (Variables|Default|GetLeftTrack) AxisValue))

(event Input|AxisEvents|InputAxisRightTrackThrottle
  (params (AxisValue :type Float%20%28single-precision%29))
  ;[1 1 1] Movement Input Binding
  (Class|TankTrack|SetThrottle (Variables|Default|GetRightTrack) AxisValue))

(event Input|AxisEvents|InputAxisForward
  (params (AxisValue :type Float%20%28single-precision%29))
  ;[1 1 1] Movement Input Binding
  (Class|TankMovementComponent|IntendMoveForvard (Variables|Default|GetTankMovement) AxisValue))

(event Input|AxisEvents|InputAxisThrowRight
  (params (AxisValue :type Float%20%28single-precision%29))
  ;[1 1 1] Movement Input Binding
  (Class|TankMovementComponent|IntendTurnRight (Variables|Default|GetTankMovement) AxisValue))

(event Input|MouseEvents|LeftMouseButton
  (params (Key :type Key%20Structure :default "None"))
  ;[1 1 1] Aim Input Binding
  (:Pressed
    (Class|Tank|Fire)))

(fn ConstructionScript)